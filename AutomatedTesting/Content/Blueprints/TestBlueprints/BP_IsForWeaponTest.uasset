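; Functional test that checks whether a pickup can be picked up with the weapon the test player pawn holds.
; PrepareTest prints the name of the pawn's current weapon.
; StartTest passes the pawn to the pickup's CanBePickedUp and finishes as Succeeded or Failed based on the result.
; Leftover unconnected nodes for ammo printing, an ammo pickup cast and zeroing current ammo never run.
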(event `self.ReceivePrepareTest`
  (`KismetSystemLibrary.PrintString` (`KismetStringLibrary.Concat_StrStr` "Prepare weapon is: " (`KismetSystemLibrary.GetDisplayName` (`ShooterCharacter.GetWeapon` (`self.Player Pawn Test Object`))))))

(event `self.ReceiveStartTest`
  (if (`ShooterPickup_Ammo.CanBePickedUp` (`self.PickUpTestObject`) (`self.Player Pawn Test Object`))
    (`self.FinishTest` "Succeeded" "This type of pick up could be picked up with this type of weapon")
    (else
      (`self.FinishTest` "Failed" "This pickup cant be picked up with this type of weapon"))))

(fn `UserConstructionScript`)