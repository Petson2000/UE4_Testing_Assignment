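; Functional test that checks that giving negative ammo, as a broken pickup would, lowers the player weapon's ammo count.
; PrepareTest validates the player test object and a BP_BrokenPickUp observation point, records current ammo and destroys the Platform actor.
; StartTest calls GiveAmmo on the weapon directly with a negative amount, then passes on a decrease and errors on an increase or no change.
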(event `self.ReceivePrepareTest`
  (if (`KismetSystemLibrary.IsValid` (`self.PlayerTestObject`))
    (cast `/Game/Blueprints/Pickups/BP_BrokenPickUp` (`self.ObservationPoint`)
      (:`then`
        (set `self.PreTestAmmo` (`ShooterWeapon.GetCurrentAmmo` (`ShooterCharacter.GetWeapon` (`self.PlayerTestObject`))))
        (`self.K2_DestroyActor` (`self.Platform`)))
      (:`CastFailed`
        (`self.FinishTest` "Default" "For the test to work the test needs the observation point to be a BP_BrokenPickUp")))
    (else
      (`self.FinishTest` "Default" "The test needs a valid player test object to work"))))

(event `self.ReceiveStartTest`
  (bind _returnvalue (`ShooterCharacter.GetWeapon` (`self.PlayerTestObject`)))
  (`ShooterWeapon.GiveAmmo` _returnvalue -50)
  (if (< (`self.PreTestAmmo`) (`ShooterWeapon.GetCurrentAmmo` _returnvalue))
    (`self.FinishTest` "Error" "The ammo count was increased even thought the pick up gives negative ammo")
    (elif (< (`ShooterWeapon.GetCurrentAmmo` (`ShooterCharacter.GetWeapon` (`self.PlayerTestObject`))) (`self.PreTestAmmo`))
      (`self.FinishTest` "Succeeded" "Ammo count was decreased due to the pick up giving negative ammo")
      (elif (== (`self.PreTestAmmo`) (`ShooterWeapon.GetCurrentAmmo` (`ShooterCharacter.GetWeapon` (`self.PlayerTestObject`))))
        (`self.FinishTest` "Error" "The ammo count wasnt updated")))))

(fn `UserConstructionScript`)