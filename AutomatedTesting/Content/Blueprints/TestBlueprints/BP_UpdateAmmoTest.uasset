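; BP_UpdateAmmoTest is a functional test that checks whether a player test object's weapon gains ammo.
; On test start it waits for FallTimer, then compares the weapon's current ammo against PreTestAmmo.
; It succeeds only if ammo has increased and ObservationPoint is valid, and otherwise fails with a message that the count was not updated.
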(event `self.ReceiveStartTest`
  (`KismetSystemLibrary.Delay` (`self.FallTimer`))
  (if (and (> (`ShooterWeapon.GetCurrentAmmo` (`ShooterCharacter.GetWeapon` (`self.PlayerTestObject`))) (`self.PreTestAmmo`)) (`KismetSystemLibrary.IsValid` (`self.ObservationPoint`)))
    (`self.FinishTest` "Succeeded" "Ammo count has changed.")
    (else
      (`self.FinishTest` "Failed" "Ammo count wasnt updated"))))

(fn `UserConstructionScript`)