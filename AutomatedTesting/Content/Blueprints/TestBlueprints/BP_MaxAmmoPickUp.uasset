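; BP_MaxAmmoPickUp is a functional test that checks an ammo pickup does not raise a player's ammo beyond the weapon's maximum.
; Test preparation fills the test player's weapon to max ammo.
; On start it waits for a fall timer, then fails if current ammo exceeds the max and succeeds otherwise.
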(event `self.ReceivePrepareTest`
  (bind _returnvalue (`ShooterCharacter.GetWeapon` (`self.PlayerTestObject`)))
  (`ShooterWeapon.SetCurrentAmmo` _returnvalue (`ShooterWeapon.GetMaxAmmo` _returnvalue)))

(event `self.ReceiveStartTest`
  (bind _playertestobject (`self.PlayerTestObject`))
  (`KismetSystemLibrary.Delay` (`self.FallTimer`))
  (if (> (`ShooterWeapon.GetCurrentAmmo` (`ShooterCharacter.GetWeapon` _playertestobject)) (`ShooterWeapon.GetMaxAmmo` (`ShooterCharacter.GetWeapon` _playertestobject)))
    (`self.FinishTest` "Failed" "Players Ammo was updated even though the player had max ammo")
    (else
      (`self.FinishTest` "Succeeded" "Ammo variable wasnt updated due to the player having max ammo"))))

(fn `UserConstructionScript`)